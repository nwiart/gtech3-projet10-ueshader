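; BP_WindBlade is a wind spell projectile that slices a test cube in two on overlap, then destroys itself.
; The box overlap accepts only the first BP_TEST_CUBE found, hides its static mesh and copies it into the cube's procedural mesh.
; That mesh is sliced along the blade's Plane component with a capped cut, and the new half simulates physics.
; The construction script sets the projectile's initial speed from Speed.
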(event OnComponentBeginOverlap(Box)
  (params (OverlappedComponent :type Primitive%20Component%20Object%20Reference) (OtherActor :type Actor%20Object%20Reference) (OtherComp :type Primitive%20Component%20Object%20Reference) (OtherBodyIndex :type Integer) (bFromSweep :type Boolean) (SweepResult :type Hit%20Result%20Structure%20%28by%20ref%29))
  (bind _returnvalue (Actor|GetComponentbyClass OtherActor "/Script/ProceduralMeshComponent.ProceduralMeshComponent"))
  (bind _returnvalue_2 (Actor|GetComponentbyClass OtherActor "/Script/Engine.StaticMeshComponent"))
  (bind _plane (Variables|Default|GetPlane))
  (bind _returnvalue_3 (Actor|GetActorOfClass "/Game/WindCharacter/Spell/Blade/BP_TEST_CUBE.BP_TEST_CUBE_C"))
  (if (== _returnvalue_3 OtherActor)
    (if (Rendering|IsVisible _returnvalue_2)
      (Rendering|SetVisibility _returnvalue_2 false false)
      (Class|KismetProceduralMeshLibrary|CopyProceduralMeshfromStaticMeshComponent _returnvalue_2 0 _returnvalue true))
    (bind _outotherhalfprocmesh (Class|KismetProceduralMeshLibrary|SliceProceduralMesh _returnvalue (Transformation|GetWorldLocation _plane) (Math|Vector|GetUpVector _plane) true "CreateNewSectionForCap" "/Game/StarterContent/Materials/M_AssetPlatform.M_AssetPlatform"))
    (Physics|SetSimulatePhysics _outotherhalfprocmesh true)
    (Actor|DestroyActor)))

(fn ConstructionScript
  (CallFunction|SetSpeed))

(fn SetSpeed
  (Variables|/Script/Engine.ProjectileMovementComponent|SetInitialSpeed (Variables|Default|GetProjectileMovement) (Variables|Default|Getspeed))
  (return))