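; Player character with a ground-only dash on Left Shift and a thunder orb spawned ahead of it on E.
; The dash overrides movement via Dash_Setup, derives speed from rate and distance, and hides the mesh behind an attached Niagara effect.
; A timeline drives forward input while player input is disabled, then restores movement, visibility and control.
; The timeline's FOV lerp has a fixed zero alpha, so FOV stays constant.
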(event EventBeginPlay
  (bind _charactermovement (Variables|Character|GetCharacterMovement))
  (bind _dashrate (Variables|Default|GetDashRate))
  (bind _charactermovement_2 (Variables|Character|GetCharacterMovement))
  (|CallParentFunction)
  (Variables|/Script/Engine.CharacterMovementComponent|SetMaxWalkSpeed _charactermovement_2 (Variables|/Script/Engine.CharacterMovementComponent|GetMaxWalkSpeed _charactermovement))
  (Variables|/Script/Engine.CharacterMovementComponent|SetMaxAcceleration _charactermovement_2 (Variables|/Script/Engine.CharacterMovementComponent|GetMaxAcceleration _charactermovement))
  (Variables|/Script/Engine.CharacterMovementComponent|SetRotationRate _charactermovement_2 (Variables|/Script/Engine.CharacterMovementComponent|GetRotationRate _charactermovement))
  (Components|Timeline|SetPlayRate (Variables|Default|GetDashTimeline) _dashrate)
  (Variables|Default|SetDashSpeed (* _dashrate (Variables|Default|GetDashDistance))))

(event Input|KeyboardEvents|LeftShift
  (params (Key :type Key%20Structure :default "None"))
  (bind _fx_location (Variables|Default|GetFX_Location))
  ;[1 1 1] Dash Logic
  (:Pressed
    (if (not (AI|Components|NavMovement|IsFalling (Variables|Character|GetCharacterMovement)))
      (Utilities|DashSetup (Variables|Default|GetDashSpeed) 99999.0 "0.000000,9999999.000000,0.000000" false)
      (Utilities|FlowControl|Delay 0.1)
      (Input|DisableInput (Game|GetPlayerController 0))
      (bind _returnvalue (Niagara|SpawnSystemAttached "/Game/Blueprints/Tristan/NS_DashFX.NS_DashFX" _fx_location "None" (Transformation|GetWorldLocation _fx_location) (Math|Rotator|MakeRotator 0.0 0.0 (.yaw (Math|Rotator|MakeRotfromX (Transformation|GetActorForwardVector)))) "KeepWorldPosition" true))
      (Variables|Default|SetDash_FX _returnvalue)
      (Timeline|DashTimeline PlayFromStart
        (:Update
          (Pawn|Input|AddMovementInput (Transformation|GetActorForwardVector) 1.0 false)
          (Camera|SetFieldOfView (Variables|Default|GetFollowCamera) (Math|Float|Lerp 9e+01 1e+02 0.0)))
        (:Finished
          (Utilities|DashSetup (Variables|Default|GetMax%20Walk%20Speed) (Variables|Default|GetMax%20Acceleration) (Variables|Default|GetRotation%20Rate) true)
          (Components|Movement|StopMovementImmediately (Variables|Character|GetCharacterMovement))
          (Input|EnableInput (Game|GetPlayerController 0))
          (Components|Activation|Deactivate (Variables|Default|GetDash_FX)))))))

(event Input|KeyboardEvents|E
  (params (Key :type Key%20Structure :default "None"))
  (:Pressed
    (Game|SpawnActorfromClass "/Game/Blueprints/Tristan/BP_ThunderOrb.BP_ThunderOrb_C" (Math|Transform|MakeTransform (+ (Transformation|GetActorLocation) (* (Transformation|GetActorForwardVector) (Variables|Default|GetOffset))) (Transformation|GetActorRotation) (Variables|Default|GetScale)) "AlwaysSpawn" "MultiplyWithRoot" 0 0)))

(fn ConstructionScript
  (|CallParentFunction))