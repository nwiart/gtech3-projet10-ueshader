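; BP_ThunderShockWave is an expanding thunder shockwave that shocks goblins it touches.
; Its sphere grows every Tick by a fixed, frame-rate-dependent step up to MaxRange, recording and shocking each overlapping BP_Goblin.
; Each new overlap spawns a BP_ThunderStorm above every recorded goblin, not just the newcomer, with its Niagara Target set to that goblin.
; After a fixed delay, it clears the shock on recorded goblins and destroys itself.
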(event OnComponentBeginOverlap(Sphere)
  (params (OverlappedComponent :type Primitive%20Component%20Object%20Reference) (OtherActor :type Actor%20Object%20Reference) (OtherComp :type Primitive%20Component%20Object%20Reference) (OtherBodyIndex :type Integer) (bFromSweep :type Boolean) (SweepResult :type Hit%20Result%20Structure%20%28by%20ref%29))
  (bind _asbp_goblin (Utilities|Casting|CastToBP_Goblin OtherActor))
  (Utilities|Array|Add (Variables|Default|GetEnemiesInRange) _asbp_goblin)
  (Variables|/Game/Blueprints/Enemy/BP_Enemy.BP_Enemy_C|SetIsShocked? _asbp_goblin true)
  (for _array_element (Variables|Default|GetEnemiesInRange)
    (if (Utilities|IsValid _array_element)
      (bind _returnvalue (Game|SpawnActorfromClass "/Game/Blueprints/Tristan/BP_ThunderStorm.BP_ThunderStorm_C" (Math|Conversions|ToTransform(Vector) (+ "0.000000,0.000000,100.000000" (Transformation|GetWorldLocation (Variables|/Script/Engine.Actor|GetRootComponent _array_element)))) "Undefined" "MultiplyWithRoot" 0 0))
      (Effects|Components|ParticleSystem|SetVectorParameter (Variables|/Game/Blueprints/Tristan/BP_ThunderStorm.BP_ThunderStorm_C|GetNiagara _returnvalue) "Target" (Transformation|GetWorldLocation (Variables|/Script/Engine.Actor|GetRootComponent _array_element))))))

(event EventBeginPlay
  (Utilities|FlowControl|Delay 1e+01)
  (for _array_element (Variables|Default|GetEnemiesInRange)
    (Utilities|IsValid _array_element
      (:Is%20Valid
        (Variables|/Game/Blueprints/Enemy/BP_Enemy.BP_Enemy_C|SetIsShocked? _array_element false))))
  (Actor|DestroyActor))

(event EventTick
  (params (DeltaSeconds :type Float%20%28single-precision%29))
  (bind _sphere (Variables|Default|GetSphere))
  (bind _returnvalue (Transformation|GetWorldScale _sphere))
  (if (< (.X (Math|Vector|BreakVector _returnvalue)) (Variables|Default|GetMaxRange))
    (Transformation|SetWorldScale3D (Variables|Default|GetSphere) (+ _returnvalue "1.000000,1.000000,1.000000"))))

(fn ConstructionScript)