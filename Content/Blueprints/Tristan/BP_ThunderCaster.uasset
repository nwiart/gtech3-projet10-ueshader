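; BP_ThunderCaster is a character Blueprint that casts a thunder orb spell on input.
; Spell 1 runs only when the character is not falling and no spell is in use, then locks movement for the cast.
; After a wind-up delay it spawns a scaled-up BP_ThunderOrb at an offset rotated to the follow camera's yaw.
; A second delay restores walking and clears the UsingSpell state.
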(event Input|EnhancedActionEvents|EnhancedInputActionIA_Spell1
  (params (ActionValue :type Boolean) (ElapsedSeconds :type Float%20%28double-precision%29) (TriggeredSeconds :type Float%20%28double-precision%29) (InputAction :type Input%20Action%20Object%20Reference :default "/Game/Blueprints/Input/Actions/IA_Spell1.IA_Spell1"))
  ;[0 0 0] Spell 1
  (if (not (or (AI|Components|NavMovement|IsFalling (Variables|Character|GetCharacterMovement)) (!= (Variables|Default|GetUsingSpell) 0)))
    (Variables|Default|SetUsingSpell 1)
    (Pawn|Components|CharacterMovement|DisableMovement (Variables|Character|GetCharacterMovement))
    (Utilities|FlowControl|Delay 1.2)
    (bind _desiredview (Class|CameraComponent|GetCameraView (Variables|Default|GetFollowCamera) 0.0))
    (Game|SpawnActorfromClass "/Game/Blueprints/Tristan/BP_ThunderOrb.BP_ThunderOrb_C" (Math|Transform|MakeTransform (+ (Transformation|GetActorLocation) (Math|Vector|RotateVector (Variables|Default|GetOrbOffset) (Math|Rotator|MakeRotator 0.0 0.0 (.yaw (Math|Conversions|RotationFromXVector (Math|Vector|GetForwardVector (.Rotation (Utilities|Struct|BreakMinimalViewInfo _desiredview)))))))) (Math|Rotator|MakeRotator 0.0 0.0 (.yaw (Math|Conversions|RotationFromXVector (Math|Vector|GetForwardVector (.Rotation (Utilities|Struct|BreakMinimalViewInfo _desiredview)))))) "5.000000,5.000000,5.000000") "AlwaysSpawn" "MultiplyWithRoot" 0 0)
    (Utilities|FlowControl|Delay 1.6)
    (Pawn|Components|CharacterMovement|SetMovementMode (Variables|Character|GetCharacterMovement) "MOVE_Walking" 0)
    (Variables|Default|SetUsingSpell 0)))

(event EventBeginPlay
  (|CallParentFunction))

(fn ConstructionScript
  (|CallParentFunction))