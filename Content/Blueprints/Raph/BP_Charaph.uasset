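; BP_Charaph is a character Blueprint that casts Katon fire spells as Niagara effects.
; CastSpell switches on a spell index: the fireball attaches to the mesh's mouth socket, while the fire tornado is handled by CastSpell2.
; CastSpell2 traces from the player pawn toward a point Range units along the follow camera's view and spawns the tornado at any blocking hit.
; The spells only spawn visual systems, with no damage logic.
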(event EventBeginPlay
  (|CallParentFunction) ; This node is disabled and will not be called.\nDrag off pins to build functionality.
)

(event Collision|EventActorBeginOverlap
  (params (OtherActor :type Actor%20Object%20Reference)))

(event EventTick
  (params (DeltaSeconds :type Float%20%28single-precision%29)))

(fn ConstructionScript
  (|CallParentFunction))

(fn CastSpell
  (params (Selected%20Spell :type Integer))
  (switch int Selected%20Spell
    (:0
      (Niagara|SpawnSystemAttached "/Game/RaphStuff/NS_KatonBouleDeFeu.NS_KatonBouleDeFeu" (Variables|Character|GetMesh) "MouthSocket" "0, 0, 0" "0, 0, 0" "KeepRelativeOffset" false))
    (:1
      (CallFunction|CastSpell2))))

(fn CastSpell2
  (bind _desiredview (Class|CameraComponent|GetCameraView (Variables|Default|GetFollowCamera) 0.0))
  (bind _outhit (Collision|LineTraceForObjects (Math|Transform|TransformLocation (Transformation|GetActorTransform (Game|Player|GetPlayerPawn 0)) "0, 0, 0") (+ (.Location (Utilities|Struct|BreakMinimalViewInfo _desiredview)) (* (Math|Vector|GetForwardVector (.Rotation (Utilities|Struct|BreakMinimalViewInfo _desiredview))) (Variables|Default|GetRange))) (Variables|Default|GetObject%20Types) false 0 "None"))
  (if (.bBlockingHit (Collision|BreakHitResult _outhit))
    (Niagara|SpawnSystematLocation "/Game/RaphStuff/NS_KatonTornadeDeFeu.NS_KatonTornadeDeFeu" (.Location (Collision|BreakHitResult _outhit)))))