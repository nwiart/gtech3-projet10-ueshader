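; Goblin enemy that chases the player once it spots a character and fades out when it dies.
; Pawn sensing filters for BP_CharacterBase, then an AI MoveTo targets the first player's pawn, whichever character was seen.
; While the life system component reports death, Tick accumulates elapsed time and feeds it to the mesh's FadeAmount parameter.
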(event OnSeePawn(PawnSensing)
  (params (Pawn :type Pawn%20Object%20Reference))
  (Utilities|Casting|CastToBP_CharacterBase Pawn)
  (CallFunction|FollowPlayer))

(event Custom|FollowPlayer
  (AI|AIMoveTo self "0, 0, 0" (Game|Player|GetPlayerPawn 0) 5e+01 false))

(event EventBeginPlay
  (|CallParentFunction))

(event EventTick
  (params (DeltaSeconds :type Float%20%28single-precision%29))
  (|CallParentFunction DeltaSeconds)
  (if (Variables|/Game/Blueprints/AC_LifeSystem.AC_LifeSystem_C|GetIsDead (Variables|Default|GetAC_LifeSystem))
    (bind _output_get (Variables|Default|SetFade (+ (Variables|Default|GetFade) DeltaSeconds)))
    (Audio|Parameter|SetFloatParameter (Variables|Character|GetMesh) "FadeAmount" _output_get :!class /Script/AudioExtensions.AudioParameterControllerInterface)))

(fn ConstructionScript
  (|CallParentFunction))