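; BP_Enemy is an enemy character that takes damage from spells and carries a health bar widget above it.
; Capsule overlaps with BP_Spell apply damage through ACLifeSystem, and death hides the bar, then detaches the controller and destroys the actor after a delay.
; Each Tick updates the bar's health, turns it toward the player's follow camera, and toggles movement and animation rate from the IsFrozen flag.
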(event OnComponentBeginOverlap(CapsuleComponent)
  (params (OverlappedComponent :type Primitive%20Component%20Object%20Reference) (OtherActor :type Actor%20Object%20Reference) (OtherComp :type Primitive%20Component%20Object%20Reference) (OtherBodyIndex :type Integer) (bFromSweep :type Boolean) (SweepResult :type Hit%20Result%20Structure%20%28by%20ref%29))
  (bind _ac_lifesystem (Variables|Default|GetAC_LifeSystem))
  (bind _asbp_spell (Utilities|Casting|CastToBP_Spell OtherActor))
  (Default|TakeDamage _ac_lifesystem (Variables|/Game/Blueprints/BP_Spell.BP_Spell_C|Getdamage _asbp_spell))
  (if (Variables|/Game/Blueprints/AC_LifeSystem.AC_LifeSystem_C|GetIsDead _ac_lifesystem)
    (CallFunction|Death)))

(event Custom|Death
  (Variables|Default|SetIsAlive? false)
  (Development|SetHiddeninGame (Variables|Default|GetLifeBar) true false)
  (Utilities|FlowControl|Delay 2.0)
  (Class|Pawn|DetachfromControllerPendingDestroy)
  (Actor|DestroyActor))

(event EventBeginPlay
  (bind _aswb_life_bar (Utilities|Casting|CastToWB_LifeBar (UserInterface|GetUserWidgetObject (Variables|Default|GetLifeBar))))
  (Variables|/Game/UI/WB_LifeBar.WB_LifeBar_C|SetMaxHealth _aswb_life_bar (Variables|/Game/Blueprints/AC_LifeSystem.AC_LifeSystem_C|GetMaxHealth (Variables|Default|GetAC_LifeSystem))))

(event EventTick
  (params (DeltaSeconds :type Float%20%28single-precision%29))
  (bind _mesh (Variables|Character|GetMesh))
  (CallFunction|UpdateLifeBar)
  (if (Variables|Default|GetIsFrozen?)
    (Pawn|Components|CharacterMovement|DisableMovement (Variables|Character|GetCharacterMovement))
    (Variables|/Script/Engine.SkeletalMeshComponent|SetGlobalAnimRateScale _mesh 0.0)
    (else
      (Pawn|Components|CharacterMovement|SetMovementMode (Variables|Character|GetCharacterMovement) "MOVE_Walking" 0)
      (Variables|/Script/Engine.SkeletalMeshComponent|SetGlobalAnimRateScale _mesh 1.0))))

(fn ConstructionScript)

(fn UpdateLifeBar
  (bind _aswb_life_bar (Utilities|Casting|CastToWB_LifeBar (UserInterface|GetUserWidgetObject (Variables|Default|GetLifeBar))))
  (bind _asbp_character_base (Utilities|Casting|CastToBP_CharacterBase (Game|Player|GetPlayerPawn 0)))
  (Default|SetHealth _aswb_life_bar (Variables|/Game/Blueprints/AC_LifeSystem.AC_LifeSystem_C|GetCurrentHealth (Variables|Default|GetAC_LifeSystem)))
  (Transformation|SetWorldRotation (Variables|Default|GetLifeBar) (Math|Rotator|FindLookatRotation (Transformation|GetActorLocation self) (Transformation|GetWorldLocation (Variables|/Game/Blueprints/BP_CharacterBase.BP_CharacterBase_C|GetFollowCamera _asbp_character_base))) false false))