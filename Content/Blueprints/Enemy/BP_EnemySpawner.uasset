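; BP_EnemySpawner is an enemy spawner that endlessly spawns BP_Goblin actors around its own location.
; From BeginPlay, a Delay of SpawnDelay loops back on itself after each spawn, with no count limit or stop condition.
; The SpawnRange sphere's scaled radius bounds random X and Y offsets, giving a square area at the spawner's height, and each goblin gets a random yaw.
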(event EventBeginPlay
  (bind _spawnrange (Variables|Default|GetSpawnRange))
  (bind _returnvalue (Components|Sphere|GetScaledSphereRadius _spawnrange))
  (bind _returnvalue_2 (- 0.0 _returnvalue))
  (Utilities|FlowControl|Delay (Variables|Default|GetSpawn%20Delay) :!label _label)
  (Game|SpawnActorfromClass "/Game/Blueprints/Enemy/BP_Goblin.BP_Goblin_C" (Math|Transform|MakeTransform (+ (Transformation|GetActorLocation) (Math|Vector|MakeVector (Math|Random|RandomFloatinRange _returnvalue_2 _returnvalue) (Math|Random|RandomFloatinRange _returnvalue_2 _returnvalue) 0.0)) (Math|Rotator|MakeRotator 0.0 0.0 (Math|Random|RandomFloatinRange 0.0 3.6e+02))) "Undefined" "MultiplyWithRoot" 0 0)
  (goto _label))

(fn ConstructionScript)