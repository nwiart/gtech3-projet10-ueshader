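; BP_ProceduaralMesh is a procedural mesh test actor in the wind character's blade spell folder that builds a colored square-based pyramid.
; The construction script creates one mesh section from hardcoded vertices, triangles, UVs and vertex colors, then creates a dynamic instance of M_Basic_Wall for it.
; On BeginPlay, it reads that section's vertices back and adds them as a convex collision mesh.
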(event EventBeginPlay
  (bind _proceduraltest (Variables|Default|GetProceduralTest))
  (bind _vertices (Class|KismetProceduralMeshLibrary|GetSectionfromProceduralMesh _proceduraltest))
  (Class|ProceduralMeshComponent|AddCollisionConvexMesh _proceduraltest _vertices))

(fn ConstructionScript
  (Class|ProceduralMeshComponent|CreateMeshSectionLinearColor (Variables|Default|GetProceduralTest) 0 (Utilities|Array|MakeArray "-100.000000,-100.000000,0.000000" "-100.000000,100.000000,0.000000" "100.000000,100.000000,0.000000" "100.000000,-100.000000,0.000000" "0.000000,0.000000,100.000000") (Utilities|Array|MakeArray 0 3 1 3 2 1 0 1 4 1 2 4 2 3 4 3 0 4) 0 (Utilities|Array|MakeArray "(X=0.000000,Y=0.000000)" "(X=0.000000,Y=0.500000)" "(X=0.500000,Y=0.500000)" "(X=0.500000,Y=0.000000)" "(X=0.250000,Y=0.250000)") 0 0 0 (Utilities|Array|MakeArray "(R=0.000000,G=1.000000,B=0.819863,A=1.000000)" "(R=0.000000,G=0.766062,B=1.000000,A=1.000000)" "(R=0.000000,G=0.497424,B=1.000000,A=1.000000)" "(R=0.000000,G=0.154264,B=1.000000,A=1.000000)" "(R=1.000000,G=0.970537,B=0.992634,A=1.000000)") 0 false false)
  (Rendering|Material|CreateDynamicMaterialInstance (Variables|Default|GetProceduralTest) 0 "/Game/StarterContent/Materials/M_Basic_Wall.M_Basic_Wall" "None" :!class /Script/Engine.PrimitiveComponent))