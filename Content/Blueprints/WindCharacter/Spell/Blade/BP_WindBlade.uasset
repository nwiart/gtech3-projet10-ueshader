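; Wind blade spell projectile that cuts goblins in half on overlap, with a sound attached from spawn.
; The construction script sets the projectile's initial speed from a Speed variable.
; On first hit, it flags the goblin as sliced, hides its skeletal mesh and copies its static mesh into a procedural mesh.
; That mesh is sliced along the blade box's plane with capped cuts, and physics is enabled on the slice result.
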(event OnComponentBeginOverlap(Box)
  (params (OverlappedComponent :type Primitive%20Component%20Object%20Reference) (OtherActor :type Actor%20Object%20Reference) (OtherComp :type Primitive%20Component%20Object%20Reference) (OtherBodyIndex :type Integer) (bFromSweep :type Boolean) (SweepResult :type Hit%20Result%20Structure%20%28by%20ref%29))
  (bind _returnvalue (Actor|GetComponentbyClass OtherActor "/Script/ProceduralMeshComponent.ProceduralMeshComponent"))
  (bind _box (Variables|Default|GetBox))
  (bind _asbp_goblin (Utilities|Casting|CastToBP_Goblin OtherActor))
  (if (not (Variables|/Game/Blueprints/Enemy/BP_Goblin.BP_Goblin_C|GetIsSliced _asbp_goblin))
    (Variables|/Game/Blueprints/Enemy/BP_Goblin.BP_Goblin_C|SetIsSliced _asbp_goblin true)
    (Rendering|SetVisibility (Actor|GetComponentbyClass OtherActor "/Script/Engine.SkeletalMeshComponent") false false)
    (Utilities|FlowControl|Delay 0.05)
    (Class|KismetProceduralMeshLibrary|CopyProceduralMeshfromStaticMeshComponent (Actor|GetComponentbyClass OtherActor "/Script/Engine.StaticMeshComponent") 0 _returnvalue true)
    (bind _outotherhalfprocmesh (Class|KismetProceduralMeshLibrary|SliceProceduralMesh _returnvalue (Transformation|GetWorldLocation _box) (Math|Vector|GetUpVector _box) true "CreateNewSectionForCap" "/Game/StarterContent/Materials/M_AssetPlatform.M_AssetPlatform"))
    (Physics|SetSimulatePhysics _outotherhalfprocmesh true)
    (Utilities|FlowControl|Delay 2.0)))

(event EventTick
  (params (DeltaSeconds :type Float%20%28single-precision%29)))

(event EventBeginPlay
  (Audio|SpawnSoundAttached "/Game/sound/cue/wind/WindBlade_Cue.WindBlade_Cue" (Variables|Default|GetDefaultSceneRoot) "None" "0, 0, 0" "0, 0, 0" "KeepRelativeOffset" false 1.0 1.0 0.0 0 0))

(fn ConstructionScript
  (CallFunction|SetSpeed))

(fn SetSpeed
  (Variables|/Script/Engine.ProjectileMovementComponent|SetInitialSpeed (Variables|Default|GetProjectileMovement) (Variables|Default|Getspeed))
  (return))