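; BP_ShockwaveWind is a wind spell actor: an expanding shockwave that repeatedly damages goblins and destroys itself ten seconds after spawning.
; Tick grows the Sphere by a fixed step per frame, so expansion depends on frame rate.
; Sphere overlaps add each BP_Goblin to AllEnemies, which is never pruned.
; A CanApplieDamage flag, re-armed through a Delay, gates periodic damage to every valid stored goblin through its ACLifeSystem component.
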(event OnComponentBeginOverlap(Sphere)
  (params (OverlappedComponent :type Primitive%20Component%20Object%20Reference) (OtherActor :type Actor%20Object%20Reference) (OtherComp :type Primitive%20Component%20Object%20Reference) (OtherBodyIndex :type Integer) (bFromSweep :type Boolean) (SweepResult :type Hit%20Result%20Structure%20%28by%20ref%29))
  (bind _asbp_goblin (Utilities|Casting|CastToBP_Goblin OtherActor))
  (Utilities|Array|Add (Variables|Default|GetAllEnemies) _asbp_goblin))

(event EventBeginPlay
  (Utilities|FlowControl|Delay 1e+01)
  (Actor|DestroyActor))

(event EventTick
  (params (DeltaSeconds :type Float%20%28single-precision%29))
  (Transformation|SetWorldScale3D (Variables|Default|GetSphere) (+ (Transformation|GetWorldScale (Variables|Default|GetSphere)) "1.000000,1.000000,1.000000"))
  (if (Variables|Default|GetcanApplieDamage)
    (for _array_element (Variables|Default|GetAllEnemies)
      (Utilities|IsValid _array_element
        (:Is%20Valid
          (Default|TakeDamage (Variables|/Game/Blueprints/Enemy/BP_Enemy.BP_Enemy_C|GetAC_LifeSystem _array_element) 5.0))))
    (Variables|Default|SetcanApplieDamage false)
    (else
      (Utilities|FlowControl|Delay 0.5)
      (Variables|Default|SetcanApplieDamage true))))

(fn ConstructionScript)