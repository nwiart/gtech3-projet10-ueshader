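; Wind character Blueprint with three input-driven spells: a forward tornado, a forward wind blade and a sandstorm ultimate.
; Each input sets UsingSpell and locks movement around timed delays, though Spell2's busy check gates nothing.
; The ultimate adds sound, a shockwave and a cooldown via CanUlt.
; Its sandstorm scatters about a hundred cacti using the storm box's extent and relative, not world, location.
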(event Input|EnhancedActionEvents|EnhancedInputActionIA_Spell1
  (params (ActionValue :type Boolean) (ElapsedSeconds :type Float%20%28double-precision%29) (TriggeredSeconds :type Float%20%28double-precision%29) (InputAction :type Input%20Action%20Object%20Reference :default "/Game/Blueprints/Input/Actions/IA_Spell1.IA_Spell1"))
  ;[1 1 1] Shoot Input
  (if (not (or (AI|Components|NavMovement|IsFalling (Variables|Character|GetCharacterMovement)) (!= (Variables|Default|GetUsingSpell) 0)))
    (Variables|Default|SetUsingSpell 1)
    (Pawn|Components|CharacterMovement|DisableMovement (Variables|Character|GetCharacterMovement))
    (Utilities|FlowControl|Delay 1.2)
    (CallFunction|SpellA)
    (Utilities|FlowControl|Delay 1.6)
    (Pawn|Components|CharacterMovement|SetMovementMode (Variables|Character|GetCharacterMovement) "MOVE_Walking" 0)
    (Variables|Default|SetUsingSpell 0)))

(event Input|EnhancedActionEvents|EnhancedInputActionIA_Spell2
  (params (ActionValue :type Boolean) (ElapsedSeconds :type Float%20%28double-precision%29) (TriggeredSeconds :type Float%20%28double-precision%29) (InputAction :type Input%20Action%20Object%20Reference :default "/Game/Blueprints/Input/Actions/IA_Spell2.IA_Spell2"))
  ;[1 1 1] Shoot Input
  (if (== (Variables|Default|GetUsingSpell) 0)
    _
    (else
      _))
  (Variables|Default|SetUsingSpell 2)
  (Pawn|Components|CharacterMovement|DisableMovement (Variables|Character|GetCharacterMovement))
  (Utilities|FlowControl|Delay 0.5)
  (CallFunction|SpellE)
  (Utilities|FlowControl|Delay 1.5)
  (Pawn|Components|CharacterMovement|SetMovementMode (Variables|Character|GetCharacterMovement) "MOVE_Walking" 0)
  (Variables|Default|SetUsingSpell 0))

(event Input|EnhancedActionEvents|EnhancedInputActionIA_Ultimate
  (params (ActionValue :type Boolean) (ElapsedSeconds :type Float%20%28double-precision%29) (TriggeredSeconds :type Float%20%28double-precision%29) (InputAction :type Input%20Action%20Object%20Reference :default "/Game/Blueprints/Input/Actions/IA_Ultimate.IA_Ultimate"))
  ;[1 1 1] Shoot Input
  (if (and (== (Variables|Default|GetUsingSpell) 0) (Variables|Default|GetCanUlt))
    (Audio|SpawnSoundAttached "/Game/sound/cue/ice/ULTGLACE_Cue.ULTGLACE_Cue" (Variables|Default|GetCapsuleComponent) "None" "0, 0, 0" "0, 0, 0" "KeepRelativeOffset" false 1.0 1.0 0.0 0 0)
    (Variables|Default|SetUsingSpell 3)
    (Pawn|Components|CharacterMovement|DisableMovement (Variables|Character|GetCharacterMovement))
    (Utilities|FlowControl|Delay 1.7)
    (Variables|Default|SetCanUlt false)
    (Game|SpawnActorfromClass "/Game/Blueprints/Francois/BP_Shockwave.BP_Shockwave_C" (Transformation|GetActorTransform) "Undefined" "MultiplyWithRoot" 0 0)
    (CallFunction|SpellR)
    (Utilities|FlowControl|Delay 1.3)
    (Pawn|Components|CharacterMovement|SetMovementMode (Variables|Character|GetCharacterMovement) "MOVE_Walking" 0)
    (Variables|Default|SetUsingSpell 0)
    (Utilities|FlowControl|Delay 3e+01)
    (Variables|Default|SetCanUlt true)))

(fn ConstructionScript)

(fn SpellA
  (Game|SpawnActorfromClass "/Game/Blueprints/WindCharacter/Spell/Tornado/BP_Tornade.BP_Tornade_C" (Math|Transform|MakeTransform (+ (Transformation|GetActorLocation) (* (Transformation|GetActorForwardVector) "100.000000,100.000000,100.000000")) (Transformation|GetActorRotation)) "Undefined" "MultiplyWithRoot" 0 0)
  (return))

(fn SpellR
  (bind _returnvalue (Game|SpawnActorfromClass "/Game/Blueprints/WindCharacter/Spell/Storm/BP_SandStorm.BP_SandStorm_C" (Math|Conversions|ToTransform(Vector) (+ (Transformation|GetActorLocation) "0.000000,0.000000,200.000000")) "Undefined" "MultiplyWithRoot" 0 0))
  (for _index (range 0 100)
    (Game|SpawnActorfromClass "/Game/Blueprints/WindCharacter/BP_CactusDeLaMortQuiTue.BP_CactusDeLaMortQuiTue_C" (Math|Conversions|ToTransform(Vector) (Math|Random|RandomPointinBoundingBox (Variables|/Script/Engine.SceneComponent|GetRelativeLocation (Variables|/Game/Blueprints/WindCharacter/Spell/Storm/BP_SandStorm.BP_SandStorm_C|GetBox _returnvalue)) (Variables|/Script/Engine.BoxComponent|GetBoxExtent (Variables|/Game/Blueprints/WindCharacter/Spell/Storm/BP_SandStorm.BP_SandStorm_C|GetBox _returnvalue)))) "Undefined" "MultiplyWithRoot" 0 0))
  (return))

(fn SpellE
  (Game|SpawnActorfromClass "/Game/Blueprints/WindCharacter/Spell/Blade/BP_WindBlade.BP_WindBlade_C" (Math|Transform|MakeTransform (+ (Transformation|GetActorLocation) (* (Transformation|GetActorForwardVector) "100.000000,100.000000,100.000000")) (Transformation|GetActorRotation)) "Undefined" "MultiplyWithRoot" 0 0)
  (return))