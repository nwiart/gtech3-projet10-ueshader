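; Ice caster character with three input-driven abilities, coordinated by a UsingSpell state.
; Spell 1 roots the caster and spawns ice spikes; Spell 2 toggles a speed boost with an ice trail.
; The ultimate spawns a shockwave, enables snow and temporarily drives material parameters on "Ice"-tagged meshes gathered by Domain overlap, feeding them the caster's position each tick.
; Domain's end overlap checks tag "None" instead of "Ice" before removal.
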(event OnComponentBeginOverlap(Domain)
  (params (OverlappedComponent :type Primitive%20Component%20Object%20Reference) (OtherActor :type Actor%20Object%20Reference) (OtherComp :type Primitive%20Component%20Object%20Reference) (OtherBodyIndex :type Integer) (bFromSweep :type Boolean) (SweepResult :type Hit%20Result%20Structure%20%28by%20ref%29))
  (bind _asstatic_mesh_component (Utilities|Casting|CastToStaticMeshComponent OtherComp))
  (if (Components|ComponentHasTag _asstatic_mesh_component "Ice")
    (Utilities|Array|Add (Variables|Default|GetMesh%20In%20Range) _asstatic_mesh_component)))

(event OnComponentEndOverlap(Domain)
  (params (OverlappedComponent :type Primitive%20Component%20Object%20Reference) (OtherActor :type Actor%20Object%20Reference) (OtherComp :type Primitive%20Component%20Object%20Reference) (OtherBodyIndex :type Integer))
  (bind _asstatic_mesh_component (Utilities|Casting|CastToStaticMeshComponent OtherComp))
  (if (Components|ComponentHasTag _asstatic_mesh_component "None")
    (Utilities|Array|RemoveItem (Variables|Default|GetMesh%20In%20Range) 0)))

(event Custom|VraimentPasUnTick
  ;[1 1 1] Ceci n'est pas un tick
  (if (Variables|Default|GetOnUltimate)
    (for _array_element (Variables|Default|GetMesh%20In%20Range)
      (Rendering|Material|SetVectorParameterValueonMaterials _array_element "Pos" (Transformation|GetActorLocation)))))

(event Input|EnhancedActionEvents|EnhancedInputActionIA_Ultimate
  (params (ActionValue :type Boolean) (ElapsedSeconds :type Float%20%28double-precision%29) (TriggeredSeconds :type Float%20%28double-precision%29) (InputAction :type Input%20Action%20Object%20Reference :default "/Game/Blueprints/Input/Actions/IA_Ultimate.IA_Ultimate"))
  ;[0 0 0] Ultimate
  (if (== (Variables|Default|GetUsingSpell) 0)
    (Audio|SpawnSoundAttached "/Game/sound/cue/ice/ULTGLACE_Cue.ULTGLACE_Cue" (Variables|Default|GetCapsuleComponent) "None" "0, 0, 0" "0, 0, 0" "KeepRelativeOffset" false 1.0 1.0 0.0 0 0)
    (Variables|Default|SetUsingSpell 3)
    (Pawn|Components|CharacterMovement|DisableMovement (Variables|Character|GetCharacterMovement))
    (Utilities|FlowControl|Delay 1.7)
    (Variables|Default|SetOnUltimate true)
    (Game|SpawnActorfromClass "/Game/Blueprints/Francois/BP_Shockwave.BP_Shockwave_C" (Transformation|GetActorTransform) "Undefined" "MultiplyWithRoot" 0 0)
    (Components|Activation|SetActive (Variables|Default|GetSnow) true false)
    (for _array_element (Variables|Default|GetMesh%20In%20Range)
      (Audio|Parameter|SetFloatParameter _array_element "OnUltimate" 1.0 :!class /Script/AudioExtensions.AudioParameterControllerInterface))
    (Utilities|FlowControl|Delay 1.3)
    (Pawn|Components|CharacterMovement|SetMovementMode (Variables|Character|GetCharacterMovement) "MOVE_Walking" 0)
    (Variables|Default|SetUsingSpell 0)
    (Utilities|FlowControl|Delay 8.7)
    (for _array_element_2 (Variables|Default|GetMesh%20In%20Range)
      (Audio|Parameter|SetFloatParameter _array_element_2 "OnUltimate" 0.0 :!class /Script/AudioExtensions.AudioParameterControllerInterface)
      (Rendering|Material|SetVectorParameterValueonMaterials _array_element_2 "Pos" "-100000.000000,-100000.000000,0.000000"))
    (Components|Activation|SetActive (Variables|Default|GetSnow) false false)
    (Variables|Default|SetOnUltimate false)))

(event Input|EnhancedActionEvents|EnhancedInputActionIA_Spell2
  (params (ActionValue :type Boolean) (ElapsedSeconds :type Float%20%28double-precision%29) (TriggeredSeconds :type Float%20%28double-precision%29) (InputAction :type Input%20Action%20Object%20Reference :default "/Game/Blueprints/Input/Actions/IA_Spell2.IA_Spell2"))
  ;[0 0 0] Spell 2
  (if (== (Math|Integer|%(Integer) (Variables|Default|GetUsingSpell) 2) 0)
    (Utilities|FlowControl|FlipFlop
      (:A
        (Variables|Default|SetUsingSpell 2)
        (Variables|/Script/Engine.CharacterMovementComponent|SetMaxWalkSpeed (Variables|Character|GetCharacterMovement) (* (Variables|/Script/Engine.CharacterMovementComponent|GetMaxWalkSpeed (Variables|Character|GetCharacterMovement)) 1.5))
        (Components|Activation|SetActive (Variables|Default|GetIceTrail) true false))
      (:B
        (Variables|/Script/Engine.CharacterMovementComponent|SetMaxWalkSpeed (Variables|Character|GetCharacterMovement) (* (Variables|/Script/Engine.CharacterMovementComponent|GetMaxWalkSpeed (Variables|Character|GetCharacterMovement)) 0.666667))
        (Variables|Default|SetUsingSpell 0)
        (Components|Activation|SetActive (Variables|Default|GetIceTrail) false false)))))

(event Input|EnhancedActionEvents|EnhancedInputActionIA_Spell1
  (params (ActionValue :type Boolean) (ElapsedSeconds :type Float%20%28double-precision%29) (TriggeredSeconds :type Float%20%28double-precision%29) (InputAction :type Input%20Action%20Object%20Reference :default "/Game/Blueprints/Input/Actions/IA_Spell1.IA_Spell1"))
  (bind _returnvalue (Transformation|GetActorTransform))
  ;[0 0 0] Spell 1
  (if (not (or (AI|Components|NavMovement|IsFalling (Variables|Character|GetCharacterMovement)) (!= (Variables|Default|GetUsingSpell) 0)))
    (Variables|Default|SetUsingSpell 1)
    (Pawn|Components|CharacterMovement|DisableMovement (Variables|Character|GetCharacterMovement))
    (Utilities|FlowControl|Delay 1.2)
    (Game|SpawnActorfromClass "/Game/Blueprints/Francois/BP_IceSpikes.BP_IceSpikes_C" (Math|Transform|MakeTransform (Math|Vector|MakeVector (.x (.location _returnvalue)) (.y (.location _returnvalue)) 0.0) (.rotation _returnvalue) "1.500000,1.500000,1.500000") "Undefined" "MultiplyWithRoot" 0 0)
    (Utilities|FlowControl|Delay 1.6)
    (Pawn|Components|CharacterMovement|SetMovementMode (Variables|Character|GetCharacterMovement) "MOVE_Walking" 0)
    (Variables|Default|SetUsingSpell 0)
    (Utilities|FlowControl|Delay 0.5)
    (Audio|SpawnSoundAttached "/Game/sound/cue/ice/IceSpell1_Cue.IceSpell1_Cue" (Variables|Default|GetCapsuleComponent) "None" "0, 0, 0" "0, 0, 0" "KeepRelativeOffset" false 1.0 1.0 0.0 0 0)))

(event EventBeginPlay
  ;[0 0 0] Deactivate Spell2 Niagara
  (|CallParentFunction)
  (Components|Activation|ToggleActive (Variables|Default|GetIceTrail))
  (Components|Activation|ToggleActive (Variables|Default|GetSnow)))

(event EventTick
  (params (DeltaSeconds :type Float%20%28single-precision%29))
  (CallFunction|VraimentPasUnTick))

(fn ConstructionScript
  (|CallParentFunction))