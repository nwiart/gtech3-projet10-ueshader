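; BP_EarthSpellUltimate is an earth ultimate spell that strikes every life-bearing actor around it, except the caster.
; On Cast it runs the parent cast, then filters its sphere's overlapping actors for those with an AC_LifeSystem component.
; For each target it line-traces down to the ground and spawns a BP_RockClapping at the hit point with random yaw.
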(event EventBeginPlay)

(event Collision|EventActorBeginOverlap
  (params (OtherActor :type Actor%20Object%20Reference)))

(event EventTick
  (params (DeltaSeconds :type Float%20%28single-precision%29)))

(fn ConstructionScript)

(fn Cast
  (params (Caster :type BP%20Character%20Base%20Object%20Reference))
  (|CallParentFunction Caster)
  ;[1 1 1] For each actor in range which has a life component (and isn't us)
  (for _array_element (Collision|GetOverlappingActors (Variables|Default|GetSphere) 0 :!class /Script/Engine.PrimitiveComponent)
    (if (!= _array_element Caster)
      (Utilities|IsValid (Actor|GetComponentbyClass _array_element "/Game/Blueprints/AC_LifeSystem.AC_LifeSystem_C")
        (:Is%20Valid
          ;[1 1 1] Line trace into the ground to spawn at ground level
          (bind (_outhit _returnvalue) (Collision|LineTraceByChannel (Transformation|GetActorLocation _array_element) (+ (Transformation|GetActorLocation _array_element) "0.000000,0.000000,-10000.000000") "TraceTypeQuery1" false (Utilities|Array|MakeArray _array_element) "None"))
          ;[1 1 1] Spawn on ground hit
          (if _returnvalue
            (Game|SpawnActorfromClass "/Game/Blueprints/Noah/BP_RockClapping.BP_RockClapping_C" (Math|Transform|MakeTransform (.Location (Collision|BreakHitResult _outhit)) (Math|Rotator|MakeRotator 0.0 0.0 (Math|Random|RandomFloatinRange -1.8e+02 1.8e+02)) "1.000000,1.000000,1.000000") "Undefined" "MultiplyWithRoot" 0 0)))))))