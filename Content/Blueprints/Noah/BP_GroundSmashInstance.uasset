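; BP_GroundSmashInstance is a short-lived ground smash attack that plays an earth spell sound as it spawns.
; A timeline sweeps DamageBox along its local X, disables its collision at the Spikes Done event, and destroys the actor when finished.
; Overlaps launch physics bodies upward with a velocity-change impulse and deal fixed damage to any other actor with an AC_LifeSystem component.
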(event OnComponentBeginOverlap(DamageBox)
  (params (OverlappedComponent :type Primitive%20Component%20Object%20Reference) (OtherActor :type Actor%20Object%20Reference) (OtherComp :type Primitive%20Component%20Object%20Reference) (OtherBodyIndex :type Integer) (bFromSweep :type Boolean) (SweepResult :type Hit%20Result%20Structure%20%28by%20ref%29))
  (bind _returnvalue (Actor|GetComponentbyClass OtherActor "/Game/Blueprints/AC_LifeSystem.AC_LifeSystem_C"))
  (Utilities|FlowControl|Sequence
    (:then_0
      (if (Utilities|Enum|Equal(Enum) (Collision|GetCollisionObjectType OtherComp) "ECC_PhysicsBody")
        (Physics|AddImpulse OtherComp "0.000000,0.000000,600.000000" "None" true)))
    (:then_1
      (if (!= OtherActor self)
        (Utilities|IsValid _returnvalue
          (:Is%20Valid
            (Default|TakeDamage _returnvalue 1e+01)))))))

(event EventBeginPlay
  (bind _damagebox (Variables|Default|GetDamageBox))
  (bind _relativelocation (Variables|/Script/Engine.SceneComponent|GetRelativeLocation _damagebox))
  (Audio|SpawnSoundAttached "/Game/sound/wave/earth/EarthSpell2_Cue.EarthSpell2_Cue" (Variables|Default|GetDefaultSceneRoot) "None" "0, 0, 0" "0, 0, 0" "KeepRelativeOffset" false 1.0 1.0 0.0 0 0)
  (bind _damage_box_x (Timeline|Timeline Play)
    (:Update
      (Transformation|SetRelativeLocation _damagebox (Math|Vector|MakeVector _damage_box_x (.y _relativelocation) (.z _relativelocation)) true false))
    (:Finished
      (Actor|DestroyActor))
    (:Spikes%20Done
      (Collision|SetCollisionEnabled (Variables|Default|GetDamageBox) "NoCollision"))))

(fn ConstructionScript)