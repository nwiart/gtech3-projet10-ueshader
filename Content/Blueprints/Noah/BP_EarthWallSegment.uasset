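; BP_EarthWallSegment is one segment of an earth wall spell that moves vertically, breaks apart and removes itself.
; On BeginPlay it plays a start sound and a single Timeline that drives the cylinder's relative Z and a dither dirt material's opacity.
; The Timeline's Explode event swaps the cylinder for a physics-simulated Geometry Collection with a destroy sound.
; The dynamic material is created on that collection, and the actor is destroyed when the Timeline finishes.
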(event EventBeginPlay
  (Audio|SpawnSoundAttached "/Game/sound/wave/earth/SpellEarth1Start_Cue.SpellEarth1Start_Cue" (Variables|Default|GetScene) "None" "0, 0, 0" "0, 0, 0" "KeepRelativeOffset" false 1.0 1.0 0.0 0 0)
  (bind (_direction _z_position _opacity) (Timeline|Timeline Play)
    (:Update
      (Transformation|SetRelativeLocation (Variables|Default|GetCylinder) (Math|Vector|MakeVector 0.0 0.0 _z_position) false false)
      (Rendering|Material|SetScalarParameterValue (Variables|Default|GetMaterialInstance) "Opacity" _opacity :!class /Script/Engine.MaterialInstanceDynamic))
    (:Finished
      (Actor|DestroyActor))
    (:Explode
      (Audio|SpawnSoundAttached "/Game/sound/wave/earth/DestroySpell1Earth_Cue.DestroySpell1Earth_Cue" (Variables|Default|GetScene) "None" "0, 0, 0" "0, 0, 0" "KeepRelativeOffset" false 1.0 1.0 0.0 0 0)
      (CallFunction|Explode))))

(fn ConstructionScript
  (bind _returnvalue (Rendering|Material|CreateDynamicMaterialInstance (Variables|Default|GetBP_EarthWall_GeometryCollection) 0 "/Game/Materials/M_DirtDither.M_DirtDither" "None" :!class /Script/Engine.PrimitiveComponent))
  (Variables|Default|SetMaterialInstance _returnvalue))

(fn Explode
  (bind _bp_earthwall_geometrycollection (Variables|Default|GetBP_EarthWall_GeometryCollection))
  (bind _cylinder (Variables|Default|GetCylinder))
  (Rendering|SetVisibility _cylinder false false)
  (Collision|SetCollisionEnabled _cylinder "NoCollision")
  (Physics|SetSimulatePhysics _bp_earthwall_geometrycollection true)
  (Rendering|SetVisibility _bp_earthwall_geometrycollection true false))