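; BP_EarthSpellWall is an earth spell that raises a wall of BP_EarthWallSegment actors when cast.
; The construction script gathers its static mesh components as spawn markers and sets their forward offset to WallSpawnRange.
; Cast calls the parent, then traces vertically at each marker to find the ground.
; Each hit spawns a segment there with random yaw to disguise repeated debris meshes.
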(event EventBeginPlay)

(fn ConstructionScript
  (bind _output_get (Variables|Default|SetSpawnLocations (Actor|GetComponentsByClass "/Script/Engine.StaticMeshComponent")))
  (for _array_element _output_get
    (Transformation|SetRelativeLocation _array_element (Math|Vector|MakeVector (Variables|Default|GetWallSpawnRange) (.y (Variables|/Script/Engine.SceneComponent|GetRelativeLocation _array_element)) (.z (Variables|/Script/Engine.SceneComponent|GetRelativeLocation _array_element))) false true)))

(fn Cast
  (params (Caster :type BP%20Character%20Base%20Object%20Reference))
  (bind _output_get (LocalVariables|SetLocal%20Caster Caster))
  (|CallParentFunction _output_get)
  (for _array_element (Variables|Default|GetSpawnLocations)
    ;[1 1 1] Line trace into the ground to determine spawn location
    (bind (_outhit _returnvalue) (Collision|LineTraceByChannel (+ (Transformation|GetWorldLocation _array_element) "0.000000,0.000000,400.000000") (+ (Transformation|GetWorldLocation _array_element) "0.000000,0.000000,-1200.000000") "TraceTypeQuery1" false 0 "None"))
    ;[1 1 1] Spawn on hit
    (if _returnvalue
      (Game|SpawnActorfromClass "/Game/Blueprints/Noah/BP_EarthWallSegment.BP_EarthWallSegment_C" (Math|Transform|MakeTransform (.Location (Collision|BreakHitResult _outhit)) (Math|Rotator|MakeRotator 0.0 0.0 (Math|Random|RandomFloatinRange -1.8e+02 1.8e+02)) "1.000000,1.000000,1.000000") "Undefined" "MultiplyWithRoot" 0 0))))