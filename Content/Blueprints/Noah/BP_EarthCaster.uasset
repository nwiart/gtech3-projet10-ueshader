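; BP_EarthCaster is an earth-themed spell caster that spawns and casts one of three spells: wall, ground smash or ultimate.
; SelectSpell calls the parent implementation, spawns the spell class matching the index, stores it as SpellInstance and attaches it to the caster.
; CastSpell calls Cast on that stored instance, if valid, passing the caster itself.
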(fn ConstructionScript)

(fn CastSpell
  (params (Selected%20Spell :type Integer))
  (bind _spellinstance (Variables|Default|GetSpellInstance))
  (Utilities|IsValid _spellinstance
    (:Is%20Valid
      (Default|Cast _spellinstance self))))

(fn SelectSpell
  (params (SpellIndex :type Integer))
  (|CallParentFunction SpellIndex)
  (bind _returnvalue (Game|SpawnActorfromClass (Utilities|Select :Index SpellIndex :Option%200 "/Game/Blueprints/Noah/BP_EarthSpellWall.BP_EarthSpellWall_C" :Option%201 "/Game/Blueprints/Noah/BP_EarthSpellGroundSmash.BP_EarthSpellGroundSmash_C" :Option%202 "/Game/Blueprints/Noah/BP_EarthSpellUltimate.BP_EarthSpellUltimate_C") (Math|Transform|MakeTransform "0, 0, 0" "0, 0, 0" "1.000000,1.000000,1.000000") "Undefined" "MultiplyWithRoot" 0 0))
  (bind _asbp_spell (Utilities|Casting|CastToBP_Spell _returnvalue))
  (bind _output_get (Variables|Default|SetSpellInstance _asbp_spell))
  (Transformation|AttachActorToActor _output_get self "None" "KeepRelative" "KeepRelative" "KeepRelative" true))