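; BP_RockClapping is a one-shot effect actor that animates a pair of hand components in a clapping motion with a particle system.
; On BeginPlay it spawns P_RockClapping at its location and plays a Timeline that drives both hands' vertical position and mirrored roll rotation.
; When the Timeline finishes, it hides both hands, waits briefly, then destroys itself.
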(event EventBeginPlay
  (bind _handleft (Variables|Default|GetHandLeft))
  (bind _handright (Variables|Default|GetHandRight))
  (Niagara|SpawnSystematLocation "/Game/Particles/P_RockClapping.P_RockClapping" (Transformation|GetActorLocation))
  (bind (_direction _rotationoffset _verticalpos) (Timeline|Timeline Play)
    (:Update
      (Utilities|FlowControl|Sequence
        (:then_0
          (Transformation|SetRelativeRotation _handright (Math|Rotator|MakeRotator _rotationoffset 0.0 0.0) false false)
          (Transformation|SetRelativeLocation _handright (Math|Vector|MakeVector 0.0 0.0 _verticalpos) false true))
        (:then_1
          (Transformation|SetRelativeRotation _handleft (Math|Rotator|MakeRotator (- 0.0 _rotationoffset) 0.0 0.0) false false)
          (Transformation|SetRelativeLocation _handleft (Math|Vector|MakeVector 0.0 0.0 _verticalpos) false true))))
    (:Finished
      (Rendering|SetVisibility (Variables|Default|GetHandLeft) false false)
      (Rendering|SetVisibility (Variables|Default|GetHandRight) false false)
      (Utilities|FlowControl|Delay 3.0)
      (Actor|DestroyActor))))

(fn ConstructionScript)