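; BP_IceCaster is an ice-caster character with two spells and an ultimate on Enhanced Input actions, tracked by a UsingSpell state.
; Spell 1 (grounded only) and the ultimate require an idle state, then lock movement while timed delays spawn BP_IceSpikes or BP_Shockwave.
; Spell 2 is a FlipFlop toggle that raises and restores walk speed, setting UsingSpell without checking it first.
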(event Input|EnhancedActionEvents|EnhancedInputActionIA_Ultimate
  (params (ActionValue :type Boolean) (ElapsedSeconds :type Float%20%28double-precision%29) (TriggeredSeconds :type Float%20%28double-precision%29) (InputAction :type Input%20Action%20Object%20Reference :default "/Game/Blueprints/Input/Actions/IA_Ultimate.IA_Ultimate"))
  ;[0 0 0] Ultimate
  (if (== (Variables|Default|GetUsingSpell) 0)
    (Variables|Default|SetUsingSpell 3)
    (Pawn|Components|CharacterMovement|DisableMovement (Variables|Character|GetCharacterMovement))
    (Utilities|FlowControl|Delay 1.7)
    (Game|SpawnActorfromClass "/Game/Blueprints/Characters/IceCaster/BP_Shockwave.BP_Shockwave_C" (Transformation|GetWorldTransform (Variables|Character|GetMesh)) "Undefined" "MultiplyWithRoot" 0 0)
    (Utilities|FlowControl|Delay 1.3)
    (Pawn|Components|CharacterMovement|SetMovementMode (Variables|Character|GetCharacterMovement) "MOVE_Walking" 0)
    (Variables|Default|SetUsingSpell 0)))

(event Input|EnhancedActionEvents|EnhancedInputActionIA_Spell1
  (params (ActionValue :type Boolean) (ElapsedSeconds :type Float%20%28double-precision%29) (TriggeredSeconds :type Float%20%28double-precision%29) (InputAction :type Input%20Action%20Object%20Reference :default "/Game/Blueprints/Input/Actions/IA_Spell1.IA_Spell1"))
  (bind _returnvalue (Transformation|GetActorTransform))
  ;[0 0 0] Spell 1
  (if (not (or (AI|Components|NavMovement|IsFalling (Variables|Character|GetCharacterMovement)) (!= (Variables|Default|GetUsingSpell) 0)))
    (Variables|Default|SetUsingSpell 1)
    (Pawn|Components|CharacterMovement|DisableMovement (Variables|Character|GetCharacterMovement))
    (Utilities|FlowControl|Delay 1.2)
    (Game|SpawnActorfromClass "/Game/Blueprints/Characters/IceCaster/BP_IceSpikes.BP_IceSpikes_C" (Math|Transform|MakeTransform (Math|Vector|MakeVector (.x (.location _returnvalue)) (.y (.location _returnvalue)) 0.0) (.rotation _returnvalue) "1.500000,1.500000,1.500000") "Undefined" "MultiplyWithRoot" 0 0)
    (Utilities|FlowControl|Delay 1.6)
    (Pawn|Components|CharacterMovement|SetMovementMode (Variables|Character|GetCharacterMovement) "MOVE_Walking" 0)
    (Variables|Default|SetUsingSpell 0)))

(event Input|EnhancedActionEvents|EnhancedInputActionIA_Spell2
  (params (ActionValue :type Boolean) (ElapsedSeconds :type Float%20%28double-precision%29) (TriggeredSeconds :type Float%20%28double-precision%29) (InputAction :type Input%20Action%20Object%20Reference :default "/Game/Blueprints/Input/Actions/IA_Spell2.IA_Spell2"))
  (Utilities|FlowControl|FlipFlop
    (:A
      (Variables|Default|SetUsingSpell 2)
      (Variables|/Script/Engine.CharacterMovementComponent|SetMaxWalkSpeed (Variables|Character|GetCharacterMovement) (* (Variables|/Script/Engine.CharacterMovementComponent|GetMaxWalkSpeed (Variables|Character|GetCharacterMovement)) 1.5)))
    (:B
      (Variables|/Script/Engine.CharacterMovementComponent|SetMaxWalkSpeed (Variables|Character|GetCharacterMovement) (* (Variables|/Script/Engine.CharacterMovementComponent|GetMaxWalkSpeed (Variables|Character|GetCharacterMovement)) 0.666667))
      (Variables|Default|SetUsingSpell 0))))

(fn ConstructionScript
  (|CallParentFunction))